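; Actor component for the dungeon interaction system that tracks a set of levers and checks whether enough of them are active.
; On BeginPlay it binds to each lever's hit event and builds a boolean array parallel to the Levers array.
; Each lever switch updates that lever's entry, recounts active levers and calls RequirementMet at the threshold, otherwise ProgressMade with the current count.
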(event `self.ReceiveBeginPlay`
  ;[1 0.6532 0.2657] Initialize Lever Count and Populate Boolean Matrix with Lever States
  (for _array_element (`self.Levers`)
    (`KismetArrayLibrary.Array_Add` (`self.BooleanMatrix`))
    (add `/Game/DungeonSystem/Interaction/Lever.LeverHit` _array_element (`|CreateDelegate` :!event `LeverSwitch`))))

(event `LeverSwitch`
  (params (`LeverActivated?` :type Boolean) (LeverRef :type "/Game/DungeonSystem/Interaction/Lever Object Reference"))
  (bind _leverprogress (`self.LeverProgress`))
  (for (_array_element _array_index) (`self.Levers`)
    ;[1 1 1] Update Boolean Matrix with Incoming data from Updating Lever
    (if (== LeverRef _array_element)
      (`KismetArrayLibrary.Array_Set` (`self.BooleanMatrix`) _array_index `LeverActivated?`)))
  ;[1 1 1] Take the Data from Boolean Matrix and Count a True Returns
  (set `self.LeverProgress` 0)
  (for _array_element_2 (`self.BooleanMatrix`)
    (if _array_element_2
      (`/Engine/EditorBlueprintResources/StandardMacros.IncrementInt` (`self.LeverProgress`))))
  (if (>= _leverprogress (`self.LeverRequirement`))
    (`self.RequirementMet`)
    (else
      (`self.ProgressMade` _leverprogress))))